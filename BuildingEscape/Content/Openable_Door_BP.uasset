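; Openable door actor that swings open and closed in response to OpenDoor's OnOpen and OnClose events.
; It stores its starting rotation on BeginPlay, then a timeline adds an animated yaw angle to that rotation.
; Opening plays the timeline and closing reverses it, while an event track on the same timeline times the door lock sound at the actor's location.
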(event OnClose(OpenDoor)
  (bind _open_angle (Timeline|Timeline_0 Reverse)
    (:Update
      (Transformation|SetActorRotation (Math|Rotator|CombineRotators (Math|Rotator|MakeRotator 0.0 0.0 _open_angle) (Variables|Default|GetInitial%20Rotation))))
    (:Sound%20Timing
      (Audio|PlaySoundatLocation "/Game/StarterContent/Audio/door-lock.door-lock" (Transformation|GetActorLocation)))))

(event OnOpen(OpenDoor)
  (bind _open_angle (Timeline|Timeline_0 Play)
    (:Update
      (Transformation|SetActorRotation (Math|Rotator|CombineRotators (Math|Rotator|MakeRotator 0.0 0.0 _open_angle) (Variables|Default|GetInitial%20Rotation))))
    (:Sound%20Timing
      (Audio|PlaySoundatLocation "/Game/StarterContent/Audio/door-lock.door-lock" (Transformation|GetActorLocation)))))

(event EventBeginPlay
  (Variables|Default|SetInitial%20Rotation (Transformation|GetActorRotation)))

(event Collision|EventActorBeginOverlap
  (params (OtherActor :type Actor%20Object%20Reference)))

(event EventTick
  (params (DeltaSeconds :type Float%20%28single-precision%29)))

(fn ConstructionScript)